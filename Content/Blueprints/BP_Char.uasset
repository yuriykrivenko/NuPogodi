(event Custom|UnpausedGame
  (bind _asgame_instance_np (Utilities|Casting|CastToGameInstanceNP (Game|GetGameInstance)))
  (Variables|/Game/Blueprints/GameInstanceNP.GameInstanceNP_C|SetWolfLeftDown _asgame_instance_np false)
  (Sprite|SetFlipbook (Variables|Default|GetSprite) (Variables|Animations|GetWolf_Left_Down)))

(event EventBeginPlay
  (bind _output_get (Variables|Default|SetTrue true))
  (bind _asgame_instance_np (Utilities|Casting|CastToGameInstanceNP (Game|GetGameInstance)))
  (Variables|/Game/Blueprints/GameInstanceNP.GameInstanceNP_C|SetWolfLeftDown _asgame_instance_np _output_get)
  (Sprite|SetFlipbook (Variables|Default|GetSprite) (Variables|Animations|GetWolf_Left_Down)))

(event Input|ActionEvents|InputActionPauseGame
  (params (Key :type Key%20Structure :default "None"))
  (:Pressed
    (bind _returnvalue (UserInterface|CreateWidget "/Game/Blueprints/PauseMenu.PauseMenu_C"))
    (bind _output_get (Variables|Default|SetPauseMenuRef _returnvalue))
    (UserInterface|Viewport|AddtoViewport _output_get 0)))

(event Input|KeyboardEvents|I
  (params (Key :type Key%20Structure :default "None"))
  (:Pressed
    (bind _asnu_pogidi_game_mode (Utilities|Casting|CastToNuPogidiGameMode (Game|GetGameMode)))
    (Default|AddPoints _asnu_pogidi_game_mode)))

(event Input|KeyboardEvents|Enter
  (params (Key :type Key%20Structure :default "None"))
  (:Pressed
    (bind _asnu_pogidi_game_mode (Utilities|Casting|CastToNuPogidiGameMode (Game|GetGameMode)))
    (Default|EndGame _asnu_pogidi_game_mode)
    (Development|PrintString "Score Saved")))

(event Input|KeyboardEvents|AnyKey
  (params (Key :type Key%20Structure :default "None"))
  (:Pressed
    (bind _output_flipbook (CallFunction|AnimStateMachine (Class|KismetInputLibrary|KeyGetDisplayName Key)))
    (Sprite|SetFlipbook (Variables|Default|GetSprite) _output_flipbook)))

(fn ConstructionScript)

(fn AnimStateMachine
  (params (KeyPressed :type Text))
  ;[1 1 1] Wolf's animation
  (switch string (Utilities|String|ToString(Text) KeyPressed)
    (:A
      (bind _output_get (Variables|Default|SetTrue true))
      (bind _asgame_instance_np (Utilities|Casting|CastToGameInstanceNP (Game|GetGameInstance)))
      (Variables|/Game/Blueprints/GameInstanceNP.GameInstanceNP_C|SetWolfLeftUp _asgame_instance_np _output_get)
      (bind _output_get_2 (Variables|Default|SetTrue false))
      (bind _output_get_3 (Variables|/Game/Blueprints/GameInstanceNP.GameInstanceNP_C|SetWolfLeftDown _asgame_instance_np _output_get_2))
      (bind _output_get_4 (Variables|/Game/Blueprints/GameInstanceNP.GameInstanceNP_C|SetWolfRightUp _asgame_instance_np _output_get_3))
      (Variables|/Game/Blueprints/GameInstanceNP.GameInstanceNP_C|SetWolfRightDown _asgame_instance_np _output_get_4)
      (Variables|Default|SetAnimationState "NewEnumerator0"))
    (:Z
      (bind _output_get_5 (Variables|Default|SetTrue true :!label _label))
      (bind _asgame_instance_np_2 (Utilities|Casting|CastToGameInstanceNP (Game|GetGameInstance)))
      (Variables|/Game/Blueprints/GameInstanceNP.GameInstanceNP_C|SetWolfLeftDown _asgame_instance_np_2 _output_get_5)
      (bind _output_get_6 (Variables|Default|SetTrue false))
      (bind _output_get_7 (Variables|/Game/Blueprints/GameInstanceNP.GameInstanceNP_C|SetWolfLeftUp _asgame_instance_np_2 _output_get_6))
      (bind _output_get_8 (Variables|/Game/Blueprints/GameInstanceNP.GameInstanceNP_C|SetWolfRightUp _asgame_instance_np_2 _output_get_7))
      (Variables|/Game/Blueprints/GameInstanceNP.GameInstanceNP_C|SetWolfRightDown _asgame_instance_np_2 _output_get_8)
      (Variables|Default|SetAnimationState "NewEnumerator1"))
    (:K
      (bind _output_get_9 (Variables|Default|SetTrue true))
      (bind _asgame_instance_np_3 (Utilities|Casting|CastToGameInstanceNP (Game|GetGameInstance)))
      (Variables|/Game/Blueprints/GameInstanceNP.GameInstanceNP_C|SetWolfRightUp _asgame_instance_np_3 _output_get_9)
      (bind _output_get_10 (Variables|Default|SetTrue false))
      (bind _output_get_11 (Variables|/Game/Blueprints/GameInstanceNP.GameInstanceNP_C|SetWolfLeftUp _asgame_instance_np_3 _output_get_10))
      (bind _output_get_12 (Variables|/Game/Blueprints/GameInstanceNP.GameInstanceNP_C|SetWolfLeftDown _asgame_instance_np_3 _output_get_11))
      (Variables|/Game/Blueprints/GameInstanceNP.GameInstanceNP_C|SetWolfRightDown _asgame_instance_np_3 _output_get_12)
      (Variables|Default|SetAnimationState "NewEnumerator2"))
    (:M
      (bind _output_get_13 (Variables|Default|SetTrue true))
      (bind _asgame_instance_np_4 (Utilities|Casting|CastToGameInstanceNP (Game|GetGameInstance)))
      (Variables|/Game/Blueprints/GameInstanceNP.GameInstanceNP_C|SetWolfRightDown _asgame_instance_np_4 _output_get_13)
      (bind _output_get_14 (Variables|Default|SetTrue false))
      (bind _output_get_15 (Variables|/Game/Blueprints/GameInstanceNP.GameInstanceNP_C|SetWolfLeftUp _asgame_instance_np_4 _output_get_14))
      (bind _output_get_16 (Variables|/Game/Blueprints/GameInstanceNP.GameInstanceNP_C|SetWolfLeftDown _asgame_instance_np_4 _output_get_15))
      (Variables|/Game/Blueprints/GameInstanceNP.GameInstanceNP_C|SetWolfRightUp _asgame_instance_np_4 _output_get_16)
      (Variables|Default|SetAnimationState "NewEnumerator3"))
    (:Left%20Mouse%20Button
      (goto _label)))
  (return (Utilities|Select :Index (Variables|Default|GetAnimationState) :NewEnumerator0 (Variables|Animations|GetWolf_Left_Up) :NewEnumerator1 (Variables|Animations|GetWolf_Left_Down) :NewEnumerator2 (Variables|Animations|GetWolf_Right_Up) :NewEnumerator3 (Variables|Animations|GetWolf_Right_Down))))