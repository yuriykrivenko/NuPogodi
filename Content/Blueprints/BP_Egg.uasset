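; BP_Egg is an egg Blueprint with four directional variants: up-left, down-left, up-right and down-right.
; BeginPlay calls SetEgg with the up-left type.
; SetEgg switches on the type to assign the matching sprite and set Score, which is identical for every variant.
; Each branch then calls SetEgg again with its own type, with no exit condition shown.
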(event Custom|Set%20Egg
  (params (Type :type Eggs_Enum%20Enum :default "NewEnumerator0"))
  (bind _eggsprite (Variables|Default|GetEggSprite))
  (switch Utilities|FlowControl|Switch|SwitchonEggs_Enum Type
    (:NewEnumerator0
      (Rendering|Components|Sprite|SetSprite _eggsprite "/Game/Sprites/Egg_UpLeft_Sprite.Egg_UpLeft_Sprite")
      (Variables|Default|SetScore 1)
      (CallFunction|SetEgg "NewEnumerator0"))
    (:NewEnumerator1
      (Rendering|Components|Sprite|SetSprite _eggsprite "/Game/Sprites/Egg_DownLeft_Sprite.Egg_DownLeft_Sprite")
      (Variables|Default|SetScore 1)
      (CallFunction|SetEgg "NewEnumerator1"))
    (:NewEnumerator2
      (Rendering|Components|Sprite|SetSprite _eggsprite "/Game/Sprites/Egg_UpRight_Sprite.Egg_UpRight_Sprite")
      (Variables|Default|SetScore 1)
      (CallFunction|SetEgg "NewEnumerator2"))
    (:NewEnumerator3
      (Rendering|Components|Sprite|SetSprite _eggsprite "/Game/Sprites/Egg_DownRight_Sprite.Egg_DownRight_Sprite")
      (Variables|Default|SetScore 1)
      (CallFunction|SetEgg "NewEnumerator3"))))

(event EventBeginPlay
  (CallFunction|SetEgg "NewEnumerator0"))

(fn ConstructionScript)