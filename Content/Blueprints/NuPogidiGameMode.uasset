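; Game mode for Nu Pogidi that tracks the player's score and keeps a persistent top-score table.
; BeginPlay loads the table from the BP_SaveGame slot, or creates and saves one from class defaults.
; AddPoints increments the score.
; EndGame inserts name and score above the first entry it ties or beats, drops the last entry to keep the table size fixed, then saves.
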(event Custom|AddPoints
  (bind _output_get (Variables|Default|SetPlayerScore (+ (Variables|Default|GetPlayerScore) 1)))
  (Development|PrintString (Utilities|String|ToString(Integer) _output_get)))

(event Custom|EndGame
  (bind _topscores_gm (Variables|Default|GetTopScores_GM))
  (bind (_newhighscore_ _topscoreindex) (CallFunction|CheckforHighscore))
  (Variables|Default|SetSlotToScoreIn _topscoreindex)
  (if _newhighscore_
    (Utilities|Array|Insert _topscores_gm (Utilities|Struct|MakeScoreInfo (Variables|Default|GetPlayerName) (Variables|Default|GetPlayerScore)) (Variables|Default|GetSlotToScoreIn))
    (Utilities|Array|RemoveIndex _topscores_gm (Utilities|Array|LastIndex _topscores_gm))
    (CallFunction|SaveGame)
    (Development|PrintString "End Game")))

(event EventBeginPlay
  (bind _returnvalue (SaveGame|DoesSaveGameExist (Variables|Default|GetMySaveGame)))
  (if _returnvalue
    (CallFunction|LoadGame)
    (Development|PrintString "Game Loaded")
    (else
      (CallFunction|SaveGame)))
  (for _array_element (Variables|Default|GetTopScores_GM)
    (Development|PrintString (Utilities|String|ToString(Integer) (.PlayerScore (Utilities|Struct|BreakScoreInfo _array_element))))))

(fn ConstructionScript)

(fn LoadGame
  (bind _returnvalue (SaveGame|LoadGamefromSlot (Variables|Default|GetMySaveGame)))
  (bind _asbp_save_game (Utilities|Casting|CastToBP_SaveGame _returnvalue))
  (bind _output_get (Variables|Default|SetSaveGameReference _asbp_save_game))
  (Variables|Default|SetTopScores_GM (Variables|/Game/Blueprints/BP_SaveGame.BP_SaveGame_C|GetTopScores _output_get))
  (Development|PrintString "Load Game"))

(fn SaveGame
  (Utilities|IsValid (Variables|Default|GetSaveGameReference)
    (:Is%20Valid
      (Variables|/Game/Blueprints/BP_SaveGame.BP_SaveGame_C|SetTopScores (Variables|Default|GetSaveGameReference) (Variables|Default|GetTopScores_GM)))
    (:Is%20Not%20Valid
      (bind _returnvalue (SaveGame|CreateSaveGameObject "/Game/Blueprints/BP_SaveGame.BP_SaveGame_C"))
      (bind _output_get (Variables|Default|SetSaveGameReference _returnvalue))
      (Variables|Default|SetTopScores_GM (Variables|/Game/Blueprints/BP_SaveGame.BP_SaveGame_C|GetTopScores _output_get))))
  (SaveGame|SaveGametoSlot (Variables|Default|GetSaveGameReference) (Variables|Default|GetMySaveGame))
  (Development|PrintString "Save Game to Slot"))

(fn CheckforHighscore
  (bind (_array_element _array_index) (Utilities|Array|ForEachLoopwithBreak (Variables|Default|GetTopScores_GM) :!label _label)
    (:LoopBody
      (if (>= (Variables|Default|GetPlayerScore) (.PlayerScore (Utilities|Struct|BreakScoreInfo _array_element)))
        (LocalVariables|SetHighScore? true)
        (goto _label Break)))
    (:Completed
      (return (LocalVariables|GetHighScore?) _array_index))))