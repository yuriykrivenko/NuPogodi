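; BP_Perches runs the core loop of a wolf egg-catching game, with game over after three strikes.
; A looping timer picks one of four perches and steps egg sprites along it using visibility toggles and delays.
; At the end, GameInstance wolf-position flags decide catch or miss.
; Catches update HUD score, rescale speed at milestones and periodically show a rabbit; misses briefly pause play, and the final one saves any high score.
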(event Custom|EggSpawn
  (bind _returnvalue (Game|GetPlayerController 0))
  (bind _strikes (Variables|Default|GetStrikes))
  (bind _chick_right_fb (Variables|Default|GetChick_Right_FB))
  (bind _chick_left_fb (Variables|Default|GetChick_Left_FB))
  ;[1 1 1] Spawn eggs
  (switch int (Math|Random|RandomIntegerinRange 0 3)
    (:0
      ;[1 1 1] Eggs sprites animation
      (Rendering|SetVisibility (Variables|Default|GetEggLeftUp1) (Variables|Default|GetVisible) false)
      (if (Variables|Default|GetIsPaused)
        (Rendering|SetVisibility (Variables|Default|GetEggLeftUp1) (Variables|Default|GetInvisible) false)
        (else
          (Audio|PlaySound2D "/Game/Materials/Sound/Blip_Cue.Blip_Cue" 1.0 1.0 0.0 0 0)
          (Utilities|FlowControl|Delay (Variables|Default|GetDelay))
          (Rendering|SetVisibility (Variables|Default|GetEggLeftUp1) (Variables|Default|GetInvisible) false)
          (Rendering|SetVisibility (Variables|Default|GetEggLeftUp2) (Variables|Default|GetVisible) false)
          (if (Variables|Default|GetIsPaused)
            (Rendering|SetVisibility (Variables|Default|GetEggLeftUp2) (Variables|Default|GetInvisible) false)
            (else
              (Audio|PlaySound2D "/Game/Materials/Sound/Blip_Cue.Blip_Cue" 1.0 1.0 0.0 0 0)
              (Utilities|FlowControl|Delay (Variables|Default|GetDelay))
              (Rendering|SetVisibility (Variables|Default|GetEggLeftUp2) (Variables|Default|GetInvisible) false)
              (Rendering|SetVisibility (Variables|Default|GetEggLeftUp3) (Variables|Default|GetVisible) false)
              (if (Variables|Default|GetIsPaused)
                (Rendering|SetVisibility (Variables|Default|GetEggLeftUp3) (Variables|Default|GetInvisible) false)
                (else
                  (Audio|PlaySound2D "/Game/Materials/Sound/Blip_Cue.Blip_Cue" 1.0 1.0 0.0 0 0)
                  (Utilities|FlowControl|Delay (Variables|Default|GetDelay))
                  (Rendering|SetVisibility (Variables|Default|GetEggLeftUp3) (Variables|Default|GetInvisible) false)
                  (Rendering|SetVisibility (Variables|Default|GetLeftUpEgg4) (Variables|Default|GetVisible) false)
                  (if (Variables|Default|GetIsPaused)
                    (Rendering|SetVisibility (Variables|Default|GetLeftUpEgg4) (Variables|Default|GetInvisible) false)
                    (else
                      (Audio|PlaySound2D "/Game/Materials/Sound/Blip_Cue.Blip_Cue" 1.0 1.0 0.0 0 0)
                      (Utilities|FlowControl|Delay (Variables|Default|GetDelay))
                      (Rendering|SetVisibility (Variables|Default|GetLeftUpEgg4) (Variables|Default|GetInvisible) false)
                      (Rendering|SetVisibility (Variables|Default|GetLeftUpEgg5) (Variables|Default|GetVisible) false)
                      (if (Variables|Default|GetIsPaused)
                        (Rendering|SetVisibility (Variables|Default|GetLeftUpEgg5) (Variables|Default|GetInvisible) false)
                        (else
                          (Audio|PlaySound2D "/Game/Materials/Sound/Blip_Cue.Blip_Cue" 1.0 1.0 0.0 0 0)
                          (Utilities|FlowControl|Delay (Variables|Default|GetDelay))
                          (Rendering|SetVisibility (Variables|Default|GetLeftUpEgg5) (Variables|Default|GetInvisible) false)
                          (bind _asgame_instance_np (Utilities|Casting|CastToGameInstanceNP (Game|GetGameInstance)))
                          (if (Variables|/Game/Blueprints/GameInstanceNP.GameInstanceNP_C|GetWolfLeftUp _asgame_instance_np)
                            (bind _foundwidgets (Widget|GetAllWidgetsOfClass "/Game/Blueprints/BP_UI_HUD.BP_UI_HUD_C" true :!label _label))
                            (Default|UpdateScore (Utilities|Array|Get(acopy) _foundwidgets))
                            (Audio|SpawnSound2D "/Game/Materials/Sound/Catch_Cue.Catch_Cue" 1.0 1.0 0.0 0)
                            (bind _result (Math|Integer|IncrementInt (Variables|/Game/Blueprints/BP_UI_HUD.BP_UI_HUD_C|GetscoreNum (Utilities|Array|Get(acopy) _foundwidgets)))
                              (:%20%20
                                (if (== _result 10)
                                  (Rendering|SetVisibility (Variables|Default|GetRabbit_FB) true false :!label _label_2)
                                  (Audio|SpawnSound2D "/Game/Materials/Sound/Bell_Cue.Bell_Cue" 1.0 1.0 0.0 0)
                                  (Variables|Default|SetRabbitCount 1)
                                  (if (== (Math|Integer|%(Integer) _result 100) 0) :!label _label_3
                                    (Variables|Default|SetAcceleration (* (Variables|Default|GetAcceleration) 2.5))
                                    (Variables|Default|SetDelay (* (Variables|Default|GetDelay) 2.5))
                                    (bind _returnvalue_2 (Utilities|Time|SetTimerbyFunctionName 0 "EggSpawn" (Variables|Default|GetAcceleration) true :!label _label_4))
                                    (Variables|Default|SetTimerHandle _returnvalue_2)
                                    (elif (== (Math|Integer|%(Integer) _result 10) 0)
                                      (Variables|Default|SetAcceleration (* (Variables|Default|GetAcceleration) 0.9))
                                      (Variables|Default|SetDelay (* (Variables|Default|GetDelay) 0.9))
                                      (goto _label_4)))
                                  (elif (== (Math|Integer|%(Integer) (- _result 91) 100) 0)
                                    (goto _label_2)
                                    (elif (>= (Variables|Default|GetRabbitCount) 1)
                                      (bind _output_get (Variables|Default|SetRabbitCount (Variables|Default|GetRabbitCount)))
                                      (bind _result_2 (Math|Integer|IncrementInt _output_get)
                                        (:%20%20
                                          (if (== _result_2 3)
                                            (Rendering|SetVisibility (Variables|Default|GetRabbit_FB) false false)
                                            (Variables|Default|SetRabbitCount 0)
                                            (goto _label_3))))
                                      (else
                                        (goto _label_3)))))))
                            (else
                              ;[1 1 1] Strikes animation
                              (Components|Timeline|SetLooping _chick_left_fb false :!label _label_5)
                              (Rendering|SetVisibility _chick_left_fb true false)
                              (Components|Timeline|PlayfromStart _chick_left_fb)
                              (Rendering|SetVisibility (Variables|Default|GetRabbit_FB) false false :!label _label_6)
                              (Variables|Default|SetRabbitCount 0)
                              ;[1 1 1] Strikes calc
                              (Variables|Default|SetIsPaused true)
                              (Utilities|Time|PauseTimerbyHandle (Variables|Default|GetTimerHandle))
                              (if (< _strikes 3)
                                (bind _result_3 (Math|Integer|IncrementInt _strikes)
                                  (:%20%20
                                    (if (== _result_3 3)
                                      ;[1 1 1] Strikes animation, game over
                                      (Rendering|SetVisibility (Variables|Default|GetChick_Strike_Sprite3) true false)
                                      (Audio|SpawnSound2D "/Game/Materials/Sound/GameOver_Cue.GameOver_Cue" 1.0 1.0 0.0 0)
                                      (Utilities|FlowControl|Delay 3.0)
                                      (Input|DisableInput (Game|GetPlayerCharacter 0) _returnvalue)
                                      (bind _returnvalue_3 (UserInterface|CreateWidget "/Game/Blueprints/GameOverWidget.GameOverWidget_C"))
                                      (UserInterface|Viewport|AddtoViewport _returnvalue_3 0)
                                      (Variables|/Script/Engine.PlayerController|SetbShowMouseCursor _returnvalue true)
                                      (Input|SetInputModeUIOnly _returnvalue _returnvalue_3 "DoNotLock")
                                      (bind _asgame_instance_np_2 (Utilities|Casting|CastToGameInstanceNP (Game|GetGameInstance)))
                                      (bind _returnvalue_4 (SaveGame|DoesSaveGameExist "HighscoreData"))
                                      (if _returnvalue_4
                                        (bind _returnvalue_5 (SaveGame|LoadGamefromSlot "HighscoreData"))
                                        (bind _output_get_2 (Variables|Default|SetSaverSubClass _returnvalue_5))
                                        (bind _asbp_endless_save_game (Utilities|Casting|CastToBP_EndlessSaveGame _output_get_2))
                                        (if (> (Variables|/Game/Blueprints/GameInstanceNP.GameInstanceNP_C|GetScore _asgame_instance_np_2) (Variables|/Game/Blueprints/BP_EndlessSaveGame.BP_EndlessSaveGame_C|GetHiscoreValue _asbp_endless_save_game))
                                          (Variables|/Game/Blueprints/BP_EndlessSaveGame.BP_EndlessSaveGame_C|SetHiscoreValue _asbp_endless_save_game (Variables|/Game/Blueprints/GameInstanceNP.GameInstanceNP_C|GetScore _asgame_instance_np_2))
                                          (SaveGame|SaveGametoSlot (Variables|Default|GetSaverSubClass) "HighscoreData"))
                                        (else
                                          (bind _returnvalue_6 (SaveGame|CreateSaveGameObject "/Game/Blueprints/BP_EndlessSaveGame.BP_EndlessSaveGame_C"))
                                          (bind _output_get_3 (Variables|Default|SetSaverSubClass _returnvalue_6))
                                          (bind _asbp_endless_save_game_2 (Utilities|Casting|CastToBP_EndlessSaveGame _output_get_3))
                                          (Variables|/Game/Blueprints/BP_EndlessSaveGame.BP_EndlessSaveGame_C|SetHiscoreValue _asbp_endless_save_game_2 (Variables|/Game/Blueprints/GameInstanceNP.GameInstanceNP_C|GetScore _asgame_instance_np_2))
                                          (SaveGame|SaveGametoSlot (Variables|Default|GetSaverSubClass) "HighscoreData")))
                                      (else
                                        (switch int _result_3
                                          (:1
                                            (Audio|SpawnSound2D "/Game/Materials/Sound/Chick_Cue.Chick_Cue" 1.0 1.0 0.0 0)
                                            (Rendering|SetVisibility (Variables|Default|GetChick_Strike_Sprite1) true false))
                                          (:2
                                            (Audio|SpawnSound2D "/Game/Materials/Sound/Chick_Cue.Chick_Cue" 1.0 1.0 0.0 0)
                                            (Rendering|SetVisibility (Variables|Default|GetChick_Strike_Sprite2) true false)))
                                        (Utilities|FlowControl|Delay 3.0)
                                        (Utilities|Time|UnpauseTimerbyHandle (Variables|Default|GetTimerHandle))
                                        (Variables|Default|SetIsPaused false)))))))))))))))))))
    (:1
      (Rendering|SetVisibility (Variables|Default|GetEggLeftDown1) (Variables|Default|GetVisible) false)
      (if (Variables|Default|GetIsPaused)
        (Rendering|SetVisibility (Variables|Default|GetEggLeftDown1) (Variables|Default|GetInvisible) false)
        (else
          (Audio|PlaySound2D "/Game/Materials/Sound/Blip_Cue.Blip_Cue" 1.0 1.0 0.0 0 0)
          (Utilities|FlowControl|Delay (Variables|Default|GetDelay))
          (Rendering|SetVisibility (Variables|Default|GetEggLeftDown1) (Variables|Default|GetInvisible) false)
          (Rendering|SetVisibility (Variables|Default|GetEggLeftDown2) (Variables|Default|GetVisible) false)
          (if (Variables|Default|GetIsPaused)
            (Rendering|SetVisibility (Variables|Default|GetEggLeftDown2) (Variables|Default|GetInvisible) false)
            (else
              (Audio|PlaySound2D "/Game/Materials/Sound/Blip_Cue.Blip_Cue" 1.0 1.0 0.0 0 0)
              (Utilities|FlowControl|Delay (Variables|Default|GetDelay))
              (Rendering|SetVisibility (Variables|Default|GetEggLeftDown2) (Variables|Default|GetInvisible) false)
              (Rendering|SetVisibility (Variables|Default|GetEggLeftDown3) (Variables|Default|GetVisible) false)
              (if (Variables|Default|GetIsPaused)
                (Rendering|SetVisibility (Variables|Default|GetEggLeftDown3) (Variables|Default|GetInvisible) false)
                (else
                  (Audio|PlaySound2D "/Game/Materials/Sound/Blip_Cue.Blip_Cue" 1.0 1.0 0.0 0 0)
                  (Utilities|FlowControl|Delay (Variables|Default|GetDelay))
                  (Rendering|SetVisibility (Variables|Default|GetEggLeftDown3) (Variables|Default|GetInvisible) false)
                  (Rendering|SetVisibility (Variables|Default|GetEggLeftDown4) (Variables|Default|GetVisible) false)
                  (if (Variables|Default|GetIsPaused)
                    (Rendering|SetVisibility (Variables|Default|GetEggLeftDown4) (Variables|Default|GetInvisible) false)
                    (else
                      (Audio|PlaySound2D "/Game/Materials/Sound/Blip_Cue.Blip_Cue" 1.0 1.0 0.0 0 0)
                      (Utilities|FlowControl|Delay (Variables|Default|GetDelay))
                      (Rendering|SetVisibility (Variables|Default|GetEggLeftDown4) (Variables|Default|GetInvisible) false)
                      (Rendering|SetVisibility (Variables|Default|GetEggLeftDown5) (Variables|Default|GetVisible) false)
                      (if (Variables|Default|GetIsPaused)
                        (Rendering|SetVisibility (Variables|Default|GetEggLeftDown5) (Variables|Default|GetInvisible) false)
                        (else
                          (Audio|PlaySound2D "/Game/Materials/Sound/Blip_Cue.Blip_Cue" 1.0 1.0 0.0 0 0)
                          (Utilities|FlowControl|Delay (Variables|Default|GetDelay))
                          (Rendering|SetVisibility (Variables|Default|GetEggLeftDown5) (Variables|Default|GetInvisible) false)
                          (bind _asgame_instance_np_3 (Utilities|Casting|CastToGameInstanceNP (Game|GetGameInstance)))
                          (if (Variables|/Game/Blueprints/GameInstanceNP.GameInstanceNP_C|GetWolfLeftDown _asgame_instance_np_3)
                            (goto _label)
                            (else
                              (goto _label_5))))))))))))))
    (:2
      (Rendering|SetVisibility (Variables|Default|GetEggRightUp1) (Variables|Default|GetVisible) false)
      (if (Variables|Default|GetIsPaused)
        (Rendering|SetVisibility (Variables|Default|GetEggRightUp1) (Variables|Default|GetInvisible) false)
        (else
          (Audio|PlaySound2D "/Game/Materials/Sound/Blip_Cue.Blip_Cue" 1.0 1.0 0.0 0 0)
          (Utilities|FlowControl|Delay (Variables|Default|GetDelay))
          (Rendering|SetVisibility (Variables|Default|GetEggRightUp1) (Variables|Default|GetInvisible) false)
          (Rendering|SetVisibility (Variables|Default|GetEggRightUp2) (Variables|Default|GetVisible) false)
          (if (Variables|Default|GetIsPaused)
            (Rendering|SetVisibility (Variables|Default|GetEggRightUp2) (Variables|Default|GetInvisible) false)
            (else
              (Audio|PlaySound2D "/Game/Materials/Sound/Blip_Cue.Blip_Cue" 1.0 1.0 0.0 0 0)
              (Utilities|FlowControl|Delay (Variables|Default|GetDelay))
              (Rendering|SetVisibility (Variables|Default|GetEggRightUp2) (Variables|Default|GetInvisible) false)
              (Rendering|SetVisibility (Variables|Default|GetEggRightUp3) (Variables|Default|GetVisible) false)
              (if (Variables|Default|GetIsPaused)
                (Rendering|SetVisibility (Variables|Default|GetEggRightUp3) (Variables|Default|GetInvisible) false)
                (else
                  (Audio|PlaySound2D "/Game/Materials/Sound/Blip_Cue.Blip_Cue" 1.0 1.0 0.0 0 0)
                  (Utilities|FlowControl|Delay (Variables|Default|GetDelay))
                  (Rendering|SetVisibility (Variables|Default|GetEggRightUp3) (Variables|Default|GetInvisible) false)
                  (Rendering|SetVisibility (Variables|Default|GetEggRightUp4) (Variables|Default|GetVisible) false)
                  (if (Variables|Default|GetIsPaused)
                    (Rendering|SetVisibility (Variables|Default|GetEggRightUp4) (Variables|Default|GetInvisible) false)
                    (else
                      (Audio|PlaySound2D "/Game/Materials/Sound/Blip_Cue.Blip_Cue" 1.0 1.0 0.0 0 0)
                      (Utilities|FlowControl|Delay (Variables|Default|GetDelay))
                      (Rendering|SetVisibility (Variables|Default|GetEggRightUp4) (Variables|Default|GetInvisible) false)
                      (Rendering|SetVisibility (Variables|Default|GetEggRightUp5) (Variables|Default|GetVisible) false)
                      (if (Variables|Default|GetIsPaused)
                        (Rendering|SetVisibility (Variables|Default|GetEggRightUp5) (Variables|Default|GetInvisible) false)
                        (else
                          (Audio|PlaySound2D "/Game/Materials/Sound/Blip_Cue.Blip_Cue" 1.0 1.0 0.0 0 0)
                          (Utilities|FlowControl|Delay (Variables|Default|GetDelay))
                          (Rendering|SetVisibility (Variables|Default|GetEggRightUp5) (Variables|Default|GetInvisible) false)
                          (bind _asgame_instance_np_4 (Utilities|Casting|CastToGameInstanceNP (Game|GetGameInstance)))
                          (if (Variables|/Game/Blueprints/GameInstanceNP.GameInstanceNP_C|GetWolfRightUp _asgame_instance_np_4)
                            (goto _label)
                            (else
                              (Components|Timeline|SetLooping _chick_right_fb false :!label _label_7)
                              (Rendering|SetVisibility _chick_right_fb true false)
                              (Components|Timeline|PlayfromStart _chick_right_fb)
                              (goto _label_6))))))))))))))
    (:3
      (Rendering|SetVisibility (Variables|Default|GetEggRightDown1) (Variables|Default|GetVisible) false)
      (if (Variables|Default|GetIsPaused)
        (Rendering|SetVisibility (Variables|Default|GetEggRightDown1) (Variables|Default|GetInvisible) false)
        (else
          (Audio|PlaySound2D "/Game/Materials/Sound/Blip_Cue.Blip_Cue" 1.0 1.0 0.0 0 0)
          (Utilities|FlowControl|Delay (Variables|Default|GetDelay))
          (Rendering|SetVisibility (Variables|Default|GetEggRightDown1) (Variables|Default|GetInvisible) false)
          (Rendering|SetVisibility (Variables|Default|GetEggRightDown2) (Variables|Default|GetVisible) false)
          (if (Variables|Default|GetIsPaused)
            (Rendering|SetVisibility (Variables|Default|GetEggRightDown2) (Variables|Default|GetInvisible) false)
            (else
              (Audio|PlaySound2D "/Game/Materials/Sound/Blip_Cue.Blip_Cue" 1.0 1.0 0.0 0 0)
              (Utilities|FlowControl|Delay (Variables|Default|GetDelay))
              (Rendering|SetVisibility (Variables|Default|GetEggRightDown2) (Variables|Default|GetInvisible) false)
              (Rendering|SetVisibility (Variables|Default|GetEggRightDown3) (Variables|Default|GetVisible) false)
              (if (Variables|Default|GetIsPaused)
                (Rendering|SetVisibility (Variables|Default|GetEggRightDown3) (Variables|Default|GetInvisible) false)
                (else
                  (Audio|PlaySound2D "/Game/Materials/Sound/Blip_Cue.Blip_Cue" 1.0 1.0 0.0 0 0)
                  (Utilities|FlowControl|Delay (Variables|Default|GetDelay))
                  (Rendering|SetVisibility (Variables|Default|GetEggRightDown3) (Variables|Default|GetInvisible) false)
                  (Rendering|SetVisibility (Variables|Default|GetEggRightDown4) (Variables|Default|GetVisible) false)
                  (if (Variables|Default|GetIsPaused)
                    (Rendering|SetVisibility (Variables|Default|GetEggRightDown4) (Variables|Default|GetInvisible) false)
                    (else
                      (Audio|PlaySound2D "/Game/Materials/Sound/Blip_Cue.Blip_Cue" 1.0 1.0 0.0 0 0)
                      (Utilities|FlowControl|Delay (Variables|Default|GetDelay))
                      (Rendering|SetVisibility (Variables|Default|GetEggRightDown4) (Variables|Default|GetInvisible) false)
                      (Rendering|SetVisibility (Variables|Default|GetEggRightDown5) (Variables|Default|GetVisible) false)
                      (if (Variables|Default|GetIsPaused)
                        (Rendering|SetVisibility (Variables|Default|GetEggRightDown5) (Variables|Default|GetInvisible) false)
                        (else
                          (Audio|PlaySound2D "/Game/Materials/Sound/Blip_Cue.Blip_Cue" 1.0 1.0 0.0 0 0)
                          (Utilities|FlowControl|Delay (Variables|Default|GetDelay))
                          (Rendering|SetVisibility (Variables|Default|GetEggRightDown5) (Variables|Default|GetInvisible) false)
                          (bind _asgame_instance_np_5 (Utilities|Casting|CastToGameInstanceNP (Game|GetGameInstance)))
                          (if (Variables|/Game/Blueprints/GameInstanceNP.GameInstanceNP_C|GetWolfRightDown _asgame_instance_np_5)
                            (goto _label)
                            (else
                              (goto _label_7))))))))))))))))

(event EventBeginPlay
  (Utilities|FlowControl|Sequence
    (:then_0
      (bind _asgame_instance_np (Utilities|Casting|CastToGameInstanceNP (Game|GetGameInstance)))
      (Variables|Default|SetAcceleration (Variables|/Game/Blueprints/GameInstanceNP.GameInstanceNP_C|GetAccelerationGlobal _asgame_instance_np)))
    (:then_1
      ;[1 1 1] Spawn eggs
      (bind _returnvalue (Utilities|Time|SetTimerbyFunctionName 0 "EggSpawn" (Variables|Default|GetAcceleration) true))
      (Variables|Default|SetTimerHandle _returnvalue))))

(fn ConstructionScript)

(fn EggSpawner)